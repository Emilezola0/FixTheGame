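; Parent AI enemy character that patrols or heads to a target location via blackboard keys and makes melee combo attacks.
; Attacks cycle through big or non-big montage arrays, with notifies reopening the attack gate and range checks on completion for repeats.
; Box traces along left and right sword sockets detect player hits, but only the left passes a damage target.
; Taking damage only prints a string.
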(event `self.ReceiveBeginPlay`
  (bind _returnvalue (`AIBlueprintHelperLibrary.GetBlackboard` null))
  (`BlackboardComponent.SetValueAsBool` _returnvalue "Patrol?" (`self.Patrol?`))
  (if (not (`self.Patrol?`))
    (`BlackboardComponent.SetValueAsVector` _returnvalue "TargetActorRandomMove" (`self.K2_GetActorLocation` (`self.Target`))))
  (set `self.Atk_IndexMax` (- (`KismetArrayLibrary.Array_Length` (`self.Atk_AnimMontageBig`)) 1))
  (bind _asbp_custom_tps (cast `/Game/Blueprints/BP_CustomTPS` (`GameplayStatics.GetPlayerCharacter` 0)))
  (set `self.Player` _asbp_custom_tps))

(event `/Game/FixTheGame_AI/AIController/BPI_AIMeleeAttack.AI Melee Atk`
  (`self.Atk`))

(event `Atk`
  (if (`self.CanAtk`)
    (set `self.CanAtk` false)
    (`/Engine/EditorBlueprintResources/StandardMacros.IsValid` self
      (:`Is Valid`
        (if (`self.IsBig? `)
          (bind _notifyname (`|PlayMontage` (`self.Mesh`) (`|GetArrayItem` (`self.Atk_AnimMontageBig`) (`self.Atk_IndexCurrent`)))
            (:`then`
              (set `self.Atk_IndexCurrent` (`KismetMathLibrary.SelectInt` (+ (`self.Atk_IndexCurrent`) 1) 0 (< (`self.Atk_IndexCurrent`) (`self.Atk_IndexMax`)))))
            (:`OnCompleted`
              (set `self.CanAtk` true)
              (if (`BlackboardComponent.GetValueAsBool` (`AIBlueprintHelperLibrary.GetBlackboard` null) "PlayerIsInMeleeRange")
                (`self.Atk`)
                (else
                  (set `self.Atk_IndexCurrent` 0))))
            (:`OnNotifyBegin`
              (switch `name` _notifyname
                (:`NPCCanCombo`
                  (set `self.CanAtk` true)))))
          (else
            (bind _notifyname_2 (`|PlayMontage` (`self.Mesh`) (`|GetArrayItem` (`self.Atk_AnimMontageNotBig`) (`self.Atk_IndexCurrent`)))
              (:`then`
                (set `self.Atk_IndexCurrent` (`KismetMathLibrary.SelectInt` (+ (`self.Atk_IndexCurrent`) 1) 0 (< (`self.Atk_IndexCurrent`) (`self.Atk_IndexMax`)))))
              (:`OnCompleted`
                (set `self.CanAtk` true)
                (if (`BlackboardComponent.GetValueAsBool` (`AIBlueprintHelperLibrary.GetBlackboard` null) "PlayerIsInMeleeRange")
                  (`self.Atk`)
                  (else
                    (set `self.Atk_IndexCurrent` 0))))
              (:`OnNotifyBegin`
                (switch `name` _notifyname_2
                  (:`NPCCanCombo`
                    (set `self.CanAtk` true)))))))))))

(event `Take Damage`
  (`KismetSystemLibrary.PrintString` "Hello" true false))

(fn `TrrigerComplexHit`
  (bind _mesh (`self.Mesh`))
  (bind _mesh_2 (`self.Mesh`))
  (bind _player (`self.Player`))
  (`|ExecutionSequence`
    (:`then_0`
      (bind _outhit (`KismetSystemLibrary.BoxTraceSingleForObjects` :`Start` (`SceneComponent.GetSocketLocation` _mesh_2 "SwordL_UpSocket") :`End` (`SceneComponent.GetSocketLocation` _mesh_2 "SwordL_DownSocket") :`HalfSize` (10.0 3.0 1.0) :`ObjectTypes` (`|MakeArray` "ObjectTypeQuery3" :!type "EObjectTypeQuery Enum") :`DrawDebugType` "ForDuration"))
      (bind _player_2 (`self.Player`)
        (:`then`
          (bind (_bblockinghit _binitialoverlap _time _distance _location _impactpoint _normal _impactnormal _physmat _hitactor) (`GameplayStatics.BreakHitResult` _outhit))
          (if (== _hitactor _player_2)
            (if (`Actor.bCanBeDamaged` _player)
              (`GameplayStatics.ApplyDamage` _player (`self.Base Damage`))
              (`NiagaraFunctionLibrary.SpawnSystemAtLocation` null _impactpoint))))
        (:`else`
          (`KismetSystemLibrary.PrintString` "not valid" true false :!label _label))))
    (:`then_1`
      (bind _outhit_2 (`KismetSystemLibrary.BoxTraceSingleForObjects` :`Start` (`SceneComponent.GetSocketLocation` _mesh "SwordR_UpSocket") :`End` (`SceneComponent.GetSocketLocation` _mesh "SwordR_DownSocket") :`HalfSize` (10.0 3.0 1.0) :`ObjectTypes` (`|MakeArray` "ObjectTypeQuery3" :!type "EObjectTypeQuery Enum") :`DrawDebugType` "ForDuration"))
      (bind _player_3 (`self.Player`)
        (:`then`
          (bind (_bblockinghit_2 _binitialoverlap_2 _time_2 _distance_2 _location_2 _impactpoint_2 _normal_2 _impactnormal_2 _physmat_2 _hitactor_2) (`GameplayStatics.BreakHitResult` _outhit_2))
          (if (== _hitactor_2 _player_3)
            (if (`Actor.bCanBeDamaged` (`self.Player`))
              (`GameplayStatics.ApplyDamage` null (`self.Base Damage`))
              (`NiagaraFunctionLibrary.SpawnSystemAtLocation` null _impactpoint_2))))
        (:`else`
          (goto _label))))))

(fn `UserConstructionScript`)