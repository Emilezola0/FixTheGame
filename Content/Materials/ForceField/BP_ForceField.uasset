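; BP_ForceField is a force field barrier that ripples when touched and disappears once its crystals are broken.
; Hits from spirit projectiles, or from the player through a resettable DoOnce, create a dynamic material instance, animate a radius from the impact point and spawn particles there.
; CrystalBreak counts down remaining crystals, then DestroyShield checks the count, fades shield visibility on a timeline and destroys the actor.
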(event `CrystalBreak`
  (bind _result (`/Engine/EditorBlueprintResources/StandardMacros.DecrementInt` (`self.CrystalToBreak`))
    (:`  `
      (if (<= _result 0)
        (`self.DestroyShield`)
        (else
          (`KismetSystemLibrary.PrintString` "Crystal " true false))))))

(event `DestroyShield`
  ;[1 1 1] Trigger Custom Event Inside Pillar
  (`self.AllRockDestroyed?`
    (:`true`
      (`/Engine/EditorBlueprintResources/StandardMacros.IsValid` (`self.MatShield`)
        (:`Is Valid`
          (bind (_direction _newtrack_0) (`Timeline|Timeline_1` :!via `PlayFromStart`)
            (:`Update`
              (`MaterialInstanceDynamic.SetScalarParameterValue` (`self.MatShield`) "Visibility" (* (- 1.0 _newtrack_0) 4.0)))
            (:`Finished`
              (`self.K2_DestroyActor` :!label _label))))
        (:`Is Not Valid`
          (goto _label))))))

(event `self.Sphere.OnComponentHit`
  (params (HitComponent :type "PrimitiveComponent Object Reference") (OtherActor :type "Actor Object Reference") (OtherComp :type "PrimitiveComponent Object Reference") (NormalImpulse :type "Vector Structure") (Hit :type "HitResult Structure (by ref)"))
  (bind (_bblockinghit _binitialoverlap _time _distance _location _impactpoint _normal _impactnormal) (`GameplayStatics.BreakHitResult` Hit))
  (bind _sphere1 (`self.Sphere1`))
  ;[1 1 1] When Hit by Actor or Projectile
  (cast `/Game/Blueprints/Spirit/BP_SpiritProjectile` OtherActor
    (:`then`
      (`/Engine/EditorBlueprintResources/StandardMacros.IsValid` _sphere1
        (:`Is Valid`
          _)))
    (:`CastFailed`
      (cast `/Game/Blueprints/BP_CustomTPS` OtherActor)
      (`/Engine/EditorBlueprintResources/StandardMacros.DoOnce` false :!label _label_2
        (:`Completed`
          _))))
  (bind _returnvalue (`PrimitiveComponent.CreateDynamicMaterialInstance` _sphere1 0 "/Game/Materials/ForceField/MI_ForceField_Inst.MI_ForceField_Inst" "None"))
  (bind _output_get (set `self.MatShield` _returnvalue))
  (`MaterialInstanceDynamic.SetVectorParameterValue` _output_get "Pos" (`KismetMathLibrary.Conv_VectorToLinearColor` _impactpoint))
  (`GameplayStatics.SpawnEmitterAtLocation` "/Game/Materials/ForceField/dotParticle.dotParticle" _impactpoint (`KismetMathLibrary.MakeRotFromX` _impactnormal))
  (bind (_direction _newtrack_0) (`Timeline|animate` :!via `PlayFromStart`)
    (:`Update`
      (`MaterialInstanceDynamic.SetScalarParameterValue` (`self.MatShield`) "Radius" (* _newtrack_0 200.0)))
    (:`Finished`
      (`KismetSystemLibrary.Delay` 1.0)
      (goto _label_2 :!via `Reset`))))

(fn `UserConstructionScript`)