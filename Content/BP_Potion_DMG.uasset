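; BP_Potion_DMG is a damage potion pickup that the player character collects by walking into it.
; On BeginPlay it spawns the NA_Aura_Damage Niagara effect at its location and keeps a reference to it.
; When a BP_CustomTPS overlaps its Box, it increments that character's damage potion count, refreshes the UI, then destroys the effect and itself.
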(event `self.ReceiveBeginPlay`
  (bind _returnvalue (`NiagaraFunctionLibrary.SpawnSystemAtLocation` "/Game/3D_Prod/Niagara/Perso/Aura/NA_Aura_Damage.NA_Aura_Damage" (`self.K2_GetActorLocation`)))
  (set `self.NewVar_0` _returnvalue))

(event `self.Box.OnComponentBeginOverlap`
  (params (OverlappedComponent :type "PrimitiveComponent Object Reference") (OtherActor :type "Actor Object Reference") (OtherComp :type "PrimitiveComponent Object Reference") (OtherBodyIndex :type Integer) (bFromSweep :type Boolean) (SweepResult :type "HitResult Structure (by ref)"))
  (bind _asbp_custom_tps (cast `/Game/Blueprints/BP_CustomTPS` OtherActor))
  (`/Engine/EditorBlueprintResources/StandardMacros.IncrementInt` (`/Game/Blueprints/BP_CustomTPS.Potion Damage Num` _asbp_custom_tps)
    (:`  `
      (`/Game/Blueprints/BP_CustomTPS.UpdateUI` _asbp_custom_tps)
      (`ActorComponent.K2_DestroyComponent` (`self.NewVar_0`))
      (`self.K2_DestroyActor`))))

(fn `UserConstructionScript`)