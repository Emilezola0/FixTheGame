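; Coin drop pickup that gives the BP_CustomTPS player a random coin amount on overlap, with a chance of a bonus potion.
; Overlap plays a sound, sets CoinsAdded, calls AddCoins and destroys the actor.
; A second sequence branch then occasionally increments an HP, Damage or Speed potion count, using nested re-rolls that favour Speed.
; The Interact event only hits an unconnected DoOnce.
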(event `/Game/Blueprints/Collectibles/BPI_Interact.Interact`
  (`/Engine/EditorBlueprintResources/StandardMacros.DoOnce` false))

(event `self.CollisionCoin.OnComponentBeginOverlap`
  (params (OverlappedComponent :type "PrimitiveComponent Object Reference") (OtherActor :type "Actor Object Reference") (OtherComp :type "PrimitiveComponent Object Reference") (OtherBodyIndex :type Integer) (bFromSweep :type Boolean) (SweepResult :type "HitResult Structure (by ref)"))
  (bind _returnvalue (`KismetMathLibrary.RandomIntegerInRange` 1 3))
  (bind _asbp_custom_tps (cast `/Game/Blueprints/BP_CustomTPS` OtherActor))
  (`GameplayStatics.PlaySound2D` "/Game/Sound/Coin/Coin_Cue.Coin_Cue" 1.0 1.0 0.0 null null)
  (`|ExecutionSequence`
    (:`then_0`
      (bind _output_get (set `/Game/Blueprints/BP_CustomTPS.Coins Added` (`KismetMathLibrary.RandomIntegerInRange` 1 15) _asbp_custom_tps))
      (`KismetSystemLibrary.PrintString` (`KismetStringLibrary.Concat_StrStr` "Coins Addes" (`KismetStringLibrary.Conv_IntToString` _output_get)) true false)
      (`/Game/Blueprints/BP_CustomTPS.Add coins` _asbp_custom_tps)
      (`self.K2_DestroyActor`))
    (:`then_1`
      (if (== (`KismetMathLibrary.RandomIntegerInRange` 1 6) 6)
        (if (== _returnvalue 1)
          (set `/Game/Blueprints/BP_CustomTPS.Potion HP Num` (+ (`/Game/Blueprints/BP_CustomTPS.Potion HP Num` _asbp_custom_tps) 1) _asbp_custom_tps)
          (elif (== _returnvalue 2)
            (set `/Game/Blueprints/BP_CustomTPS.Potion Damage Num` (+ (`/Game/Blueprints/BP_CustomTPS.Potion Damage Num` _asbp_custom_tps) 1) _asbp_custom_tps)
            (else
              (set `/Game/Blueprints/BP_CustomTPS.Potion Speed Num` (+ (`/Game/Blueprints/BP_CustomTPS.Potion Speed Num` _asbp_custom_tps) 1) _asbp_custom_tps))))))))

(fn `UserConstructionScript`)