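; BP_DeathCameraActor is a camera actor that shows the player's death from above.
; On its Death event it sweeps to a point above the BP_CustomTPS player character, pitches straight down, and blends the player controller's view to itself.
; After the blend and a short hold, it calls DeathMessage on the master game instance.
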(event `/Game/Blueprints/Death/BPI_Death.Death`
  (bind _blend_time (`self.Blend Time`))
  (bind _asbp_custom_tps (cast `/Game/Blueprints/BP_CustomTPS` (`GameplayStatics.GetPlayerCharacter` 0)))
  (set `self.As BP Custom TPS` _asbp_custom_tps)
  (bind _as_bp_custom_tps (`self.As BP Custom TPS`)
    (:`then`
      (bind _returnvalue_location (`KismetMathLibrary.BreakTransform` (`self.GetTransform` _as_bp_custom_tps)))
      (`self.K2_SetActorTransform` (`KismetMathLibrary.MakeTransform` (+ _returnvalue_location (0.0 0.0 450.0)) (struct :`Pitch` -90.0)) true)
      (`PlayerController.SetViewTargetWithBlend` (`GameplayStatics.GetPlayerController` 0) self _blend_time "VTBlend_Linear" 0.0 false)
      (`KismetSystemLibrary.Delay` (+ _blend_time 3.0))
      (message `/Game/Blueprints/Death/BPI_Death.Death` (`/Game/Core/BP_MyFunctionLibrary.getGameInstance_Master`)))
    (:`else`)))

(fn `UserConstructionScript`)