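; BP_SpiritProjectile is a spirit projectile that damages and knocks back AI enemies, acting only on its first hit.
; On BeginPlay it caches a single BP_FTG_AI_Parent actor as its Enemy.
; While that Enemy is valid, a hit AI is launched along its reversed forward vector with random strength.
; Damage, read from the player's BP_CustomTPS character, applies only if the hit actor is the cached Enemy.
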(event `self.ReceiveBeginPlay`
  (bind _returnvalue (`GameplayStatics.GetActorOfClass` "/Game/FixTheGame_AI/Chara/BP_FTG_AI_Parent.BP_FTG_AI_Parent_C"))
  (set `self.Enemy` _returnvalue))

(event `self.ReceiveHit`
  (params (MyComp :type "PrimitiveComponent Object Reference") (Other :type "Actor Object Reference") (OtherComp :type "PrimitiveComponent Object Reference") (bSelfMoved :type Boolean) (HitLocation :type "Vector Structure") (HitNormal :type "Vector Structure") (NormalImpulse :type "Vector Structure") (Hit :type "HitResult Structure (by ref)"))
  (if (not (`self.HaveBounce?`))
    (set `self.HaveBounce?` true)
    (bind _enemy (`self.Enemy`)
      (:`then`
        (bind _asbp_ftg_ai_parent (cast `/Game/FixTheGame_AI/Chara/BP_FTG_AI_Parent` Other)
          (:`then`
            (`Character.LaunchCharacter` _asbp_ftg_ai_parent (* (`self.GetActorForwardVector` _asbp_ftg_ai_parent) (* (`KismetMathLibrary.RandomFloatInRange` 50.0 100.0) -1.0)) false false))
          (:`CastFailed`
            _))
        (if (== _enemy Other)
          (bind _asbp_custom_tps (cast `/Game/Blueprints/BP_CustomTPS` (`GameplayStatics.GetPlayerCharacter` 0)))
          (`GameplayStatics.ApplyDamage` _enemy (`/Game/Blueprints/BP_CustomTPS.Damage` _asbp_custom_tps))))
      (:`else`))))

(fn `UserConstructionScript`)