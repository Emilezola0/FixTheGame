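; Crystal pillar actor that triggers a level cinematic when hit by a spirit projectile.
; On BeginPlay it flags its BP_CrystalRotationDmg child actor as a reward crystal.
; When a BP_SpiritProjectile overlaps its Box, it calls CallLevelCinematique on the BP_CustomTPS player character.
; It then destroys the Box component, so the trigger fires only once.
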(event `self.ReceiveBeginPlay`
  (bind _asbp_crystal_rotation_dmg (cast `/Game/CrystalStone/BP_CrystalRotationDmg` (`ChildActorComponent.ChildActor` (`self.ChildActor`))))
  (set `/Game/CrystalStone/BP_CrystalRotationDmg.IsRewardCrystal?` true _asbp_crystal_rotation_dmg))

(event `self.Box.OnComponentBeginOverlap`
  (params (OverlappedComponent :type "PrimitiveComponent Object Reference") (OtherActor :type "Actor Object Reference") (OtherComp :type "PrimitiveComponent Object Reference") (OtherBodyIndex :type Integer) (bFromSweep :type Boolean) (SweepResult :type "HitResult Structure (by ref)"))
  (cast `/Game/Blueprints/Spirit/BP_SpiritProjectile` OtherActor)
  (bind _asbp_custom_tps (cast `/Game/Blueprints/BP_CustomTPS` (`GameplayStatics.GetPlayerCharacter` 0)))
  (`/Game/Blueprints/BP_CustomTPS.LevelCinematique` _asbp_custom_tps)
  (`ActorComponent.K2_DestroyComponent` (`self.Box`)))

(fn `UserConstructionScript`)