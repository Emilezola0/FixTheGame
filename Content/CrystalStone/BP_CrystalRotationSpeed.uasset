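; Breakable crystal that spirit projectiles shatter, notifying its linked force field unless it is a reward crystal.
; A projectile overlapping the box enables physics on the geometry collection and calls CrystalBreak on the force field.
; A projectile hit on the collection spawns an MF_Crystal at the actor's transform, passes it a directional magnitude and triggers it.
; The hit counter increments, but the magnitude always comes from the first array entry.
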(event `ActorIsDestroy`
  ;[1 1 1] When actor is destroyed
  (if (not (`self.IsRewardCrystal?`))
    (`/Game/Materials/ForceField/BP_ForceField.CrystalBreak` (`self.ForceFieldLinked`))))

(event `self.ReceiveBeginPlay`
  (set `self.Index` 0))

(event `self.Cristal_GeometryCollection.OnComponentHit`
  (params (HitComponent :type "PrimitiveComponent Object Reference") (OtherActor :type "Actor Object Reference") (OtherComp :type "PrimitiveComponent Object Reference") (NormalImpulse :type "Vector Structure") (Hit :type "HitResult Structure (by ref)"))
  (cast `/Game/Blueprints/Spirit/BP_SpiritProjectile` OtherActor)
  (bind _returnvalue (`|SpawnActorFromClass` "/Game/Chaos/MF_Crystal.MF_Crystal_C" (`self.GetTransform`) "Undefined" "OverrideRootScale" null null))
  (set `/Engine/EditorResources/FieldNodes/FS_MasterField.DirectionalMagnitude` (`|GetArrayItem` (`self.ArrayMagnitude`)) _returnvalue)
  (`/Engine/EditorBlueprintResources/StandardMacros.IncrementInt` (`self.Index`)
    (:`  `
      (`/Engine/EditorResources/FieldNodes/FS_MasterField.CE_Trigger` _returnvalue))))

(event `self.Box.OnComponentBeginOverlap`
  (params (OverlappedComponent :type "PrimitiveComponent Object Reference") (OtherActor :type "Actor Object Reference") (OtherComp :type "PrimitiveComponent Object Reference") (OtherBodyIndex :type Integer) (bFromSweep :type Boolean) (SweepResult :type "HitResult Structure (by ref)"))
  (cast `/Game/Blueprints/Spirit/BP_SpiritProjectile` OtherActor)
  (`PrimitiveComponent.SetSimulatePhysics` (`self.Cristal_GeometryCollection`) true)
  (`self.ActorIsDestroy`))

(fn `UserConstructionScript`)