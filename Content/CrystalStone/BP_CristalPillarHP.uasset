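; Pillar actor carrying a BP_CrystalRotationHP child actor, which it flags as a reward crystal on BeginPlay.
; When a BP_SpiritProjectile overlaps its Box, it triggers the level cinematic on the player's BP_CustomTPS character and grants a random amount of coins.
; The Box is destroyed during that hit, so the cinematic and coin reward fire only once.
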(event `self.ReceiveBeginPlay`
  (bind _asbp_crystal_rotation_hp (cast `/Game/CrystalStone/BP_CrystalRotationHP` (`ChildActorComponent.ChildActor` (`self.ChildActor`))))
  (set `/Game/CrystalStone/BP_CrystalRotationHP.IsRewardCrystal?` true _asbp_crystal_rotation_hp))

(event `self.Box.OnComponentBeginOverlap`
  (params (OverlappedComponent :type "PrimitiveComponent Object Reference") (OtherActor :type "Actor Object Reference") (OtherComp :type "PrimitiveComponent Object Reference") (OtherBodyIndex :type Integer) (bFromSweep :type Boolean) (SweepResult :type "HitResult Structure (by ref)"))
  (cast `/Game/Blueprints/Spirit/BP_SpiritProjectile` OtherActor)
  (bind _asbp_custom_tps (cast `/Game/Blueprints/BP_CustomTPS` (`GameplayStatics.GetPlayerCharacter` 0)))
  (`/Game/Blueprints/BP_CustomTPS.LevelCinematique` _asbp_custom_tps)
  (`ActorComponent.K2_DestroyComponent` (`self.Box`))
  (set `/Game/Blueprints/BP_CustomTPS.Current Coins` (+ (`/Game/Blueprints/BP_CustomTPS.Current Coins` _asbp_custom_tps) (`KismetMathLibrary.RandomIntegerInRange` 20 40)) _asbp_custom_tps)
  (`/Game/Blueprints/BP_CustomTPS.Add coins` _asbp_custom_tps))

(fn `UserConstructionScript`)